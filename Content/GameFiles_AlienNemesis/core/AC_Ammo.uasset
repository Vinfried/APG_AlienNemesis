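; Actor component that tracks weapon ammo as a clip and a reserve pool, clamping every change to valid bounds.
; Using ammo subtracts a per-use cost from the clip, while pickups or other additions raise the reserve up to its maximum.
; Reserve reload sets the clip from the reserve count alone, ignoring leftover rounds, then deducts the missing amount from the reserve.
; A simple reload sets the clip directly to a supplied amount.
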(fn UseClipAmmo
  (Variables|Default|SetClip (Math|Integer|Clamp(Integer) (- (Variables|Default|GetClip) (Variables|Default|GetAmmoPerUse)) 0 (Variables|Default|GetClip))))

(fn ReloadClipfromReserve
  (LocalVariables|SetLPreviousClip (Variables|Default|GetClip))
  (Variables|Default|SetClip (Math|Integer|Clamp(Integer) (Variables|Default|GetReserve) 0 (Variables|Default|GetMaxClip)))
  (Variables|Default|SetReserve (- (Variables|Default|GetReserve) (Math|Integer|Clamp(Integer) (- (Variables|Default|GetMaxClip) (LocalVariables|GetLPreviousClip)) 0 (Variables|Default|GetReserve)))))

(fn ReloadClipSimple
  (params (AmmoToAdd :type Integer))
  (Variables|Default|SetClip (Math|Integer|Clamp(Integer) AmmoToAdd 0 (Variables|Default|GetMaxClip))))

(fn AddReserveAmmo
  (params (Amount :type Integer))
  (Variables|Default|SetReserve (Math|Integer|Clamp(Integer) (+ (Variables|Default|GetReserve) Amount) 0 (Variables|Default|GetMaxReserve))))